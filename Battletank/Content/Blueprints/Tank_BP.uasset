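; Player-drivable tank pawn Blueprint that wires input to its aiming, movement and camera components.
; On BeginPlay it hands the barrel and turret meshes to TankAiming and the two tracks to TankMovement.
; Input drives tracks either directly by per-track throttle or through TankMovement's forward and turn intents, and Fire calls TankAiming.
; Aim axes orbit the camera by yawing an azimuth gimbal and pitching the spring arm.
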(event `self.ReceiveBeginPlay`
  (`TankAimingComponent.Initialise` (`self.TankAiming`) (`self.BarrelSMC`) (`self.TurretSMC`))
  (`TankMovementComponent.Initialise` (`self.TankMovement`) (`self.Left Track`) (`self.Right Track`)))

(event `InputAction|Fire`
  (params (Key :type "Key Structure"))
  ;[1 1 1] Tank Input Binding
  (:`Pressed`
    (`TankAimingComponent.Fire` (`self.TankAiming`))))

(event `InputAxis|LeftTrackThrottle`
  (params (AxisValue :type "Float (single-precision)"))
  ;[1 1 1] Tank Input Binding
  (if (!= AxisValue 0.0)
    (`TankTrackSMC.SetThrottle` (`self.Left Track`) AxisValue)))

(event `InputAxis|AimAzimuth`
  (params (AxisValue :type "Float (single-precision)"))
  ;[1 1 1] Camera input binding
  ;;[1 1 1] Change camera on azimuth
  (`SceneComponent.K2_AddLocalRotation` (`self.Azimuth Gimbal`) (`KismetMathLibrary.MakeRotator` 0.0 0.0 AxisValue) false false))

(event `InputAxis|RightTrackThrottle`
  (params (AxisValue :type "Float (single-precision)"))
  ;[1 1 1] Tank Input Binding
  (if (!= AxisValue 0.0)
    (`TankTrackSMC.SetThrottle` (`self.Right Track`) AxisValue)))

(event `InputAxis|AimAltitude`
  (params (AxisValue :type "Float (single-precision)"))
  ;[1 1 1] Camera input binding
  ;;[1 1 1] Change camera on altitude
  (`SceneComponent.K2_AddLocalRotation` (`self.SpringArm`) (`KismetMathLibrary.MakeRotator` 0.0 AxisValue) false false))

(event `InputAxis|MoveForward`
  (params (AxisValue :type "Float (single-precision)"))
  ;[1 1 1] Tank Input Binding
  (if (!= AxisValue 0.0)
    (`TankMovementComponent.IntendMoveForward` (`self.TankMovement`) AxisValue)))

(event `InputAxis|TurnRight`
  (params (AxisValue :type "Float (single-precision)"))
  ;[1 1 1] Tank Input Binding
  (if (!= AxisValue 0.0)
    (`TankMovementComponent.IntendTurnRight` (`self.TankMovement`) AxisValue)))

(fn `UserConstructionScript`)